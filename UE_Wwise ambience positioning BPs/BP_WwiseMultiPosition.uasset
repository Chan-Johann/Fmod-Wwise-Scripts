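; Wwise ambience actor that plays one sound event as multiple sources placed along a spline.
; On BeginPlay it gathers the world positions of the spline points and moves the Ak component to the first, used for room and reverb containment.
; It passes the array to SetMultiplePositions in MultiSources mode, then posts the associated event.
; Tick draws a debug sphere at the spline's closest point to the player and prints that distance.
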(event `self.ReceiveBeginPlay`
  (bind _ak_soundsource (`self.Ak_SoundSource`))
  (bind _spline (`self.Spline`))
  ;[1 1 1] Clear spline points positions array
  (`KismetArrayLibrary.Array_Clear` (`self.Spline Points`))
  ;[1 1 1] Loop on all spline points and store their world position in an array
  (for _index (range (+ (`SplineComponent.GetNumberOfSplinePoints` _spline) 1))
    (`KismetArrayLibrary.Array_Add` (`self.Spline Points`) (`KismetMathLibrary.MakeTransform` (`SplineComponent.GetLocationAtSplinePoint` _spline _index "World"))))
  ;[1 1 1] Move the component to one of the spline point positions. This position will be used for rooms and reverb volumes containment.
  (`SceneComponent.K2_SetWorldLocation` (`self.Ak_SoundSource`) (.location (`|GetArrayItem` (`self.Spline Points`))) false true)
  ;[1 1 1] Pray Wwise will set it correctly, tho it should work only on spline points, not between
  (`AkGameplayStatics.SetMultiplePositions` _ak_soundsource (`self.Spline Points`) "MultiSources")
  (`AkComponent.PostAssociatedAkEvent` :`self` _ak_soundsource))

(event `self.ReceiveTick`
  (params (DeltaSeconds :type "Float (single-precision)"))
  (bind _returnvalue (`self.K2_GetActorLocation` (`GameplayStatics.GetPlayerPawn` 0)))
  (bind _returnvalue_2 (`KismetSystemLibrary.GetDisplayName` (`AkGameObject.AkAudioEvent` (`self.Ak_SoundSource`))))
  (bind _returnvalue_3 (`SplineComponent.FindLocationClosestToWorldLocation` (`self.Spline`) _returnvalue "World"))
  ;[1 0.9248 0.5865] Debug
  (`KismetSystemLibrary.DrawDebugSphere` _returnvalue_3 60.0 12 (struct :`R` 0.090404 :`G` 0.240329 :`B` 1.0 :`A` 1.0))
  (`KismetSystemLibrary.PrintString` (`KismetStringLibrary.Concat_StrStr` "Distance to: " _returnvalue_2 (`KismetStringLibrary.Conv_DoubleToString` (`KismetMathLibrary.Vector_Distance` _returnvalue_3 _returnvalue))) true true (struct :`R` 0.048608 :`B` 1.0 :`A` 1.0) 2.0 (`KismetStringLibrary.Conv_StringToName` _returnvalue_2)))

(fn `UserConstructionScript`)