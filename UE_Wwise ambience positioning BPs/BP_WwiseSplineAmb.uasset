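; Actor that positions a Wwise ambient sound along a spline, following the point closest to the first player's pawn.
; BeginPlay moves the Ak component onto the spline before posting its event, avoiding audible jumps, and destroys the actor if that component is invalid.
; Tick teleports the source to the closest spline point each frame.
; Tick also draws a debug sphere there and prints the distance to the player, keyed by event name.
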(event `self.ReceiveBeginPlay`
  (bind _ak_soundsource (`self.Ak_SoundSource`))
  ;[1 1 1] Moving component to correct position before we post sound to avoid weird moving ambient across the map
  (`SceneComponent.K2_SetWorldLocation` _ak_soundsource (`SplineComponent.FindLocationClosestToWorldLocation` (`self.Spline`) (`self.K2_GetActorLocation` (`GameplayStatics.GetPlayerPawn` 0)) "World") false true)
  (if (`KismetSystemLibrary.IsValid` _ak_soundsource)
    (`AkComponent.PostAssociatedAkEvent` :`self` _ak_soundsource)
    (else
      (`KismetSystemLibrary.PrintString` "No Wwise Event Assigned")
      (`self.K2_DestroyActor`))))

(event `self.ReceiveTick`
  (params (DeltaSeconds :type "Float (single-precision)"))
  (bind _ak_soundsource (`self.Ak_SoundSource`))
  (bind _returnvalue (`self.K2_GetActorLocation` (`GameplayStatics.GetPlayerPawn` 0)))
  (bind _returnvalue_2 (`KismetSystemLibrary.GetDisplayName` (`AkGameObject.AkAudioEvent` _ak_soundsource)))
  (bind _returnvalue_3 (`SplineComponent.FindLocationClosestToWorldLocation` (`self.Spline`) _returnvalue "World"))
  ;[1 1 1] Update Sound Source position
  (`SceneComponent.K2_SetWorldLocation` _ak_soundsource _returnvalue_3 false true)
  ;[1 0.9321 0.6159] Debug
  (`KismetSystemLibrary.DrawDebugSphere` _returnvalue_3 60.0 12 (struct :`R` 0.090404 :`G` 0.240329 :`B` 1.0 :`A` 1.0))
  (`KismetSystemLibrary.PrintString` (`KismetStringLibrary.Concat_StrStr` "Distance to: " _returnvalue_2 (`KismetStringLibrary.Conv_DoubleToString` (`KismetMathLibrary.Vector_Distance` _returnvalue_3 _returnvalue))) true true (struct :`R` 0.048608 :`B` 1.0 :`A` 1.0) 2.0 (`KismetStringLibrary.Conv_StringToName` _returnvalue_2)))

(fn `UserConstructionScript`)